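; BP_Paddle_Bot is an AI-controlled paddle that tracks the ball along the world X axis.
; An UpdateBallRef event receives the ball to follow.
; Each Tick, while that reference is valid, it moves toward the ball's X position at constant PaddleSpeed using VInterpToConstant, keeping its own Y and Z.
; The move is swept, so blocking collision can stop the paddle.
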(event `Update Ball Ref`
  (params (BallRef :type "/Game/Blueprints/Actors/BP_Ball Object Reference"))
  (set `self.Ball Ref` BallRef))

(event `self.ReceiveTick`
  (params (DeltaSeconds :type "Float (single-precision)"))
  (bind (_returnvalue_x _returnvalue_y _returnvalue_z) (`KismetMathLibrary.BreakVector` (`self.K2_GetActorLocation`)))
  (bind _returnvalue_x_2 (`KismetMathLibrary.BreakVector` (`self.K2_GetActorLocation` (`self.Ball Ref`))))
  (`self.Ball Ref`
    (:`then`
      (`self.K2_SetActorLocation` (`KismetMathLibrary.VInterpTo_Constant` (`self.K2_GetActorLocation`) (`KismetMathLibrary.MakeVector` _returnvalue_x_2 _returnvalue_y _returnvalue_z) DeltaSeconds (`self.PaddleSpeed`)) true))
    (:`else`)))

(fn `UserConstructionScript`)