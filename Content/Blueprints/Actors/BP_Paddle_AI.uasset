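; BP_Paddle_AI is an AI-controlled paddle that follows the ball along the X axis.
; On BeginPlay it finds the first actor tagged "Ball" and stores it through the UpdateBallRef event, printing a warning if none is found.
; Each Tick it moves toward the ball's X at a constant PaddleSpeed with VInterpToConstant and a swept move, keeping its own Y and Z.
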(event `Update Ball Ref`
  (params (BallRef :type "/Game/Blueprints/Actors/BP_Ball Object Reference"))
  (set `self.Ball Ref` BallRef))

(event `self.ReceiveBeginPlay`
  (bind _outactors (`GameplayStatics.GetAllActorsWithTag` "Ball"))
  (bind _output (`|GetArrayItem` _outactors))
  (if (`KismetSystemLibrary.IsValid` _output)
    (bind _asbp_ball (cast `/Game/Blueprints/Actors/BP_Ball` _output))
    (`self.Update Ball Ref` _asbp_ball)
    (else
      (`KismetSystemLibrary.PrintString` "Ball Not Found!"))))

(event `self.ReceiveTick`
  (params (DeltaSeconds :type "Float (single-precision)"))
  (bind (_returnvalue_x _returnvalue_y _returnvalue_z) (`KismetMathLibrary.BreakVector` (`self.K2_GetActorLocation`)))
  (bind _returnvalue_x_2 (`KismetMathLibrary.BreakVector` (`self.K2_GetActorLocation` (`self.Ball Ref`))))
  (`self.Ball Ref`
    (:`then`
      (`self.K2_SetActorLocation` (`KismetMathLibrary.VInterpTo_Constant` (`self.K2_GetActorLocation`) (`KismetMathLibrary.MakeVector` _returnvalue_x_2 _returnvalue_y _returnvalue_z) DeltaSeconds (`self.PaddleSpeed`)) true))
    (:`else`)))

(fn `UserConstructionScript`)