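; BP_PongGameMode is the game mode for a Pong game that decides when a match is won.
; On each score change it plays a goal sound at its own location and compares the player and AI scores against WinScoreNum, checking the player first.
; When either side reaches that score, it pauses the game and shows the WBP_GameFinished widget, flagged with whether the player won.
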(event `self.ReceiveBeginPlay`)

(event `self.OnScoreChanged`
  (params (NewPlayerScore :type Integer) (NewAIScore :type Integer))
  (bind _winscorenum (`self.WinScoreNum`))
  (`GameplayStatics.PlaySoundAtLocation` "/Game/SFX/Ponggoal_Cue.Ponggoal_Cue" (`self.K2_GetActorLocation`) (struct) 1.0 1.0 0.0 null null null null)
  (if (>= NewPlayerScore _winscorenum)
    (`GameplayStatics.SetGamePaused` true)
    (bind _returnvalue (`|CreateWidget` "/Game/Widgets/WBP_GameFinished.WBP_GameFinished_C" null true))
    (`UserWidget.AddToViewport` _returnvalue 0)
    (elif (>= NewAIScore _winscorenum)
      (`GameplayStatics.SetGamePaused` true)
      (bind _returnvalue_2 (`|CreateWidget` "/Game/Widgets/WBP_GameFinished.WBP_GameFinished_C"))
      (`UserWidget.AddToViewport` _returnvalue_2 0))))

(fn `UserConstructionScript`)